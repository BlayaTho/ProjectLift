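; Elevator actor that travels to a floor when called, or to a random different floor when the first-person character steps in.
; Construction script builds per-floor meshes and BP_CallLift child actors linked back to it, randomizing lift, player start and plane heights.
; MoveComponentTo drives the cabin, with duration scaled by floors travelled.
; A timeline swings both doors, and a timer closes them after inactivity.
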(event OnComponentBeginOverlap(Box)
  (params (OverlappedComponent :type Primitive%20Component%20Object%20Reference) (OtherActor :type Actor%20Object%20Reference) (OtherComp :type Primitive%20Component%20Object%20Reference) (OtherBodyIndex :type Integer) (bFromSweep :type Boolean) (SweepResult :type Hit%20Result%20Structure%20%28by%20ref%29))
  (Utilities|Casting|CastToBP_FirstPersonCharacter OtherActor)
  (if (not (Variables|Default|GetisMoving))
    (CallFunction|OpenCloseDoor true)
    (bind _output_get (Variables|Default|SetEtageToMove (Math|Random|RandomInteger (Variables|Default|GetNumbersFloors)) :!label _label))
    (if (== _output_get (Variables|Default|GetEtageAscenseur))
      (goto _label)
      (else
        (Utilities|FlowControl|Delay 1.0)
        (Variables|Default|SetisMoving true)
        (Utilities|Time|ClearandInvalidateTimerbyHandle (Variables|Default|GetTimerInactivity))
        (Components|MoveComponentTo (Variables|Default|GetLift) (Math|Vector|MakeVector 0.0 0.0 (* (Variables|Default|GetEtageToMove) 1000)) "0, 0, 0" false false (* (Math|Float|Absolute(Float) (- (Variables|Default|GetEtageToMove) (Variables|Default|GetEtageAscenseur))) 2.5) false)
        (Variables|Default|SetEtageAscenseur (Variables|Default|GetEtageToMove))
        (CallFunction|OpenCloseDoor false)
        (Variables|Default|SetisMoving false)))))

(event Custom|CloseDoorInactivity
  (if (not (Variables|Default|GetisMoving))
    (bind _lerp (Timeline|Timeline ReverseFromEnd)
      (:Update
        (Transformation|SetRelativeRotation (Variables|Default|GetSM_Lift02Door01) (Math|Rotator|MakeRotator 0.0 0.0 (Math|Float|Lerp 0.0 -25.0 _lerp)) false false)
        (Transformation|SetRelativeRotation (Variables|Default|GetSM_Lift02Door02) (Math|Rotator|MakeRotator 0.0 0.0 (Math|Float|Lerp 0.0 25.0 _lerp)) false false))
      (:Finished
        (if (not (== (.yaw (Variables|/Script/Engine.SceneComponent|GetRelativeRotation (Variables|Default|GetSM_Lift02Door01))) 0.0))
          (Utilities|FlowControl|DoOnce false
            (:Completed
              (bind _returnvalue (Utilities|Time|SetTimerbyEvent (delegate Custom|CloseDoorInactivity) 3.0))
              (Variables|Default|SetTimerInactivity _returnvalue))))))))

(event Custom|JoinMeAscenseur
  (params (EtageCall :type Integer))
  (if (== EtageCall (Variables|Default|GetEtageAscenseur))
    (CallFunction|OpenCloseDoor false)
    (else
      (CallFunction|OpenCloseDoor true)
      (Variables|Default|SetEtageToMove EtageCall)
      (Utilities|Time|ClearandInvalidateTimerbyHandle (Variables|Default|GetTimerInactivity))
      (Components|MoveComponentTo (Variables|Default|GetLift) (Math|Vector|MakeVector 0.0 0.0 (* (Variables|Default|GetEtageToMove) 1000)) "0, 0, 0" false false (* (Math|Float|Absolute(Float) (- (Variables|Default|GetEtageToMove) (Variables|Default|GetEtageAscenseur))) 2.5) false)
      (Variables|Default|SetEtageAscenseur (Variables|Default|GetEtageToMove))
      (CallFunction|OpenCloseDoor false)
      (Variables|Default|SetisMoving false))))

(event Custom|OpenCloseDoor
  (params (Close? :type Boolean))
  (Utilities|FlowControl|Sequence
    (:then_0
      (if Close?
        (bind _lerp (Timeline|Timeline ReverseFromEnd)
          (:Update
            (Transformation|SetRelativeRotation (Variables|Default|GetSM_Lift02Door01) (Math|Rotator|MakeRotator 0.0 0.0 (Math|Float|Lerp 0.0 -25.0 _lerp)) false false)
            (Transformation|SetRelativeRotation (Variables|Default|GetSM_Lift02Door02) (Math|Rotator|MakeRotator 0.0 0.0 (Math|Float|Lerp 0.0 25.0 _lerp)) false false))
          (:Finished
            (if (not (== (.yaw (Variables|/Script/Engine.SceneComponent|GetRelativeRotation (Variables|Default|GetSM_Lift02Door01))) 0.0))
              (Utilities|FlowControl|DoOnce false :!label _label
                (:Completed
                  (bind _returnvalue (Utilities|Time|SetTimerbyEvent (delegate Custom|CloseDoorInactivity) 3.0))
                  (Variables|Default|SetTimerInactivity _returnvalue))))))
        (else
          (Timeline|Timeline PlayFromStart))))
    (:then_1
      (goto _label Reset))))

(fn ConstructionScript
  (Transformation|SetWorldLocation (Variables|/Script/Engine.Actor|GetRootComponent (Variables|Default|GetPlayerStartREF)) (Math|Vector|MakeVector 0.0 4.6e+02 (Math|Conversions|ToFloat(Integer) (+ (* (Math|Random|RandomInteger (Variables|Default|GetNumbersFloors)) 1000) 100))) false false)
  (bind _output_get (Variables|Default|SetEtageAscenseur (Math|Random|RandomInteger (Variables|Default|GetNumbersFloors))))
  (Transformation|SetRelativeLocation (Variables|Default|GetLift) (Math|Vector|MakeVector 0.0 0.0 (Math|Conversions|ToFloat(Integer) (* _output_get 1000))) false false)
  (Transformation|SetRelativeLocation (Variables|Default|GetPlane) (Math|Vector|MakeVector 0.0 9.1e+02 (+ (* (Math|Random|RandomInteger (Variables|Default|GetNumbersFloors)) 1000) 120)) false false)
  (for _index (range 0 (Variables|Default|GetNumbersFloors))
    (AddComponent|AddStaticMeshComponent false (Math|Transform|MakeTransform (Math|Vector|MakeVector 0.0 4.6e+02 (Math|Conversions|ToFloat(Integer) (* _index 1000)))))
    (AddComponent|AddStaticMeshComponent false (Math|Transform|MakeTransform (Math|Vector|MakeVector 0.0 0.0 (Math|Conversions|ToFloat(Integer) (* _index 1000)))))
    (AddComponent|AddStaticMeshComponent false (Math|Transform|MakeTransform (Math|Vector|MakeVector 0.0 0.0 (+ (Math|Conversions|ToFloat(Integer) (* _index 1000)) 5e+02))))
    (bind _returnvalue (AddComponent|AddChildActorComponent false (Math|Transform|MakeTransform (Math|Vector|MakeVector -97.0 -2e+01 (+ (Math|Conversions|ToFloat(Integer) (* _index 1000)) 1.3e+02)))))
    (bind _asbp_call_lift (Utilities|Casting|CastToBP_CallLift (Variables|/Script/Engine.ChildActorComponent|GetChildActor _returnvalue)))
    (Variables|/Game/Lift/Blueprint/BP_CallLift.BP_CallLift_C|SetIndexFloor _asbp_call_lift _index)
    (Variables|/Game/Lift/Blueprint/BP_CallLift.BP_CallLift_C|SetliftREF _asbp_call_lift self)))